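; Player controller that creates the HUD and tracks a player lives count.
; BeginPlay creates the BP_Hud widget and adds it to the viewport.
; Pressing J subtracts one from PlayerLives, clamped at zero.
; The HUD's owning player comes from a cast to SideOpPlayerController that is never executed, and Tick and the construction script are empty.
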(event EventBeginPlay
  (bind _returnvalue (UserInterface|CreateWidget "/Game/HUD/BP_Hud.BP_Hud_C" (stale _asside_op_player_controller)))
  (UserInterface|Viewport|AddtoViewport _returnvalue 0))

(event EventTick
  (params (DeltaSeconds :type Float%20%28single-precision%29)))

(event Input|KeyboardEvents|J
  (:Pressed
    (if (< (- (Variables|Default|GetPlayerLives) 1) 0)
      (Variables|Default|SetPlayerLives 0)
      (else
        (Variables|Default|SetPlayerLives (- (Variables|Default|GetPlayerLives) 1))))))

(fn ConstructionScript)