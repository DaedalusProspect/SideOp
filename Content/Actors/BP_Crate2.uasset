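; A breakable crate actor that grants XP to the player who breaks it.
; When Destroyable is set, each end overlap on DestroyCollisionBox, from any actor, lowers HitsToDestroy.
; At zero it casts that actor to SideOpCharacter, adds XPtoGive to its SideOpPlayerState and destroys itself.
; If either cast fails on that last hit, the crate stays at zero and can no longer break.
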(event `self.ReceiveBeginPlay`)

(event `self.ReceiveActorBeginOverlap`
  (params (OtherActor :type "Actor Object Reference")))

(event `self.ReceiveTick`
  (params (DeltaSeconds :type "Float (single-precision)")))

(event `self.DestroyCollisionBox.OnComponentEndOverlap`
  (params (OtherActor :type "Actor Object Reference") (OtherComp :type "PrimitiveComponent Object Reference") (OtherBodyIndex :type Integer))
  (bind _hitstodestroy (`self.HitsToDestroy`))
  (if (`self.bDestroyable`)
    (if (> _hitstodestroy 0)
      (bind _output_get (set `self.HitsToDestroy` (- _hitstodestroy 1)))
      (if (== _output_get 0)
        (bind _asside_op_character (cast `SideOpCharacter` OtherActor))
        (bind _asside_op_player_state (cast `SideOpPlayerState` (`Pawn.PlayerState` _asside_op_character)))
        (`SideOpPlayerState.AddXP` _asside_op_player_state (`self.XPtoGive`))
        (`self.K2_DestroyActor`)))))

(fn `UserConstructionScript`)